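; BP_Molecule represents a molecule and shows its summary data in an on-screen info panel.
; InitialiseAtomWidget creates a WBP_MoleculeDisplay, fills its text fields from the title, timestamp, comments, atom and bond counts and chirality flag, then adds it to the viewport.
; EndPlay removes that widget from its parent, so the panel leaves with the molecule.
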(event EventEndPlay
  (params (EndPlayReason :type EEndPlayReason%20Enum :default "Destroyed"))
  (Widget|RemovefromParent (Variables|Default|GetMolDisplayWidget)))

(event EventInitialiseAtomWidget
  (bind _returnvalue (UserInterface|CreateWidget "/Game/Widgets/WBP_MoleculeDisplay.WBP_MoleculeDisplay_C"))
  (Variables|Default|SetMolDisplayWidget _returnvalue)
  (Utilities|FlowControl|Sequence
    (:then_0
      (Rendering|Components|TextRender|SetText (Variables|/Game/Widgets/WBP_MoleculeDisplay.WBP_MoleculeDisplay_C|GetNameField (Variables|Default|GetMolDisplayWidget)) (Utilities|Text|ToText(String) (Variables|Default|GetTitle))))
    (:then_1
      (Rendering|Components|TextRender|SetText (Variables|/Game/Widgets/WBP_MoleculeDisplay.WBP_MoleculeDisplay_C|GetTimestampField (Variables|Default|GetMolDisplayWidget)) (Utilities|Text|ToText(String) (Variables|Default|GetTimestamp))))
    (:then_2
      (Rendering|Components|TextRender|SetText (Variables|/Game/Widgets/WBP_MoleculeDisplay.WBP_MoleculeDisplay_C|GetCommentsField (Variables|Default|GetMolDisplayWidget)) (Utilities|Text|ToText(String) (Variables|Default|GetComments))))
    (:then_3
      (Rendering|Components|TextRender|SetText (Variables|/Game/Widgets/WBP_MoleculeDisplay.WBP_MoleculeDisplay_C|GetAtomsField (Variables|Default|GetMolDisplayWidget)) (Utilities|Text|ToText(Integer) (Variables|Default|GetAtomCount))))
    (:then_4
      (Rendering|Components|TextRender|SetText (Variables|/Game/Widgets/WBP_MoleculeDisplay.WBP_MoleculeDisplay_C|GetBondsField (Variables|Default|GetMolDisplayWidget)) (Utilities|Text|ToText(Integer) (Variables|Default|GetBondCount))))
    (:then_5
      (if (Variables|Default|GetIsChiral)
        (Variables|Default|SetChiralText "True")
        (else
          (Variables|Default|SetChiralText "False")))
      (Rendering|Components|TextRender|SetText (Variables|/Game/Widgets/WBP_MoleculeDisplay.WBP_MoleculeDisplay_C|GetChiralField (Variables|Default|GetMolDisplayWidget)) (Variables|Default|GetChiralText)))
    (:then_6
      (UserInterface|Viewport|AddtoViewport (Variables|Default|GetMolDisplayWidget) 0))))

(fn ConstructionScript)