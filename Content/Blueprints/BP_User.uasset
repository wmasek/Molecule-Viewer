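; BP_User is the player pawn for an atom viewer, a free-flying camera with a file selector and on-screen widgets created at BeginPlay.
; Tick checks the right mouse button: holding it hides the cursor, enables look and FloatingPawnMovement along camera vectors, and fades the prompt widgets accordingly.
; Select traces under the cursor for AtomComponents, currently only printing a message, and Quit exits the game.
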(event EventBeginPlay
  (bind _asplayer_controller (Utilities|Casting|CastToPlayerController (Pawn|GetController)))
  (Utilities|FlowControl|Sequence
    (:then_0
      (bind _returnvalue (UserInterface|CreateWidget "/Game/Widgets/WBP_FileSelector.WBP_FileSelector_C" _asplayer_controller))
      (UserInterface|Viewport|AddtoViewport _returnvalue 0))
    (:then_1
      (bind _returnvalue_2 (UserInterface|CreateWidget "/Game/Widgets/WBP_MousePrompt.WBP_MousePrompt_C" _asplayer_controller))
      (bind _output_get (Variables|Default|SetMousePromptWidget _returnvalue_2))
      (UserInterface|Viewport|AddtoViewport _output_get 0))
    (:then_2
      (bind _returnvalue_3 (UserInterface|CreateWidget "/Game/Widgets/WBP_ControlsDisplay.WBP_ControlsDisplay_C"))
      (bind _output_get_2 (Variables|Default|SetControlsDisplayWidget _returnvalue_3))
      (UserInterface|Viewport|AddtoViewport _output_get_2 0))
    (:then_3
      (bind _returnvalue_4 (UserInterface|CreateWidget "/Game/Widgets/WBP_AtomDisplay.WBP_AtomDisplay_C"))
      (bind _output_get_3 (Variables|Default|SetAtomDisplayWidget _returnvalue_4))
      (UserInterface|Viewport|AddtoViewport _output_get_3 0))))

(event EventTick
  (params (DeltaSeconds :type Float%20%28single-precision%29))
  (bind _returnvalue (Game|GetPlayerController 0))
  (if (Game|Player|IsInputKeyDown (Game|GetPlayerController 0) "RightMouseButton")
    (Variables|/Script/Engine.PlayerController|SetbShowMouseCursor _returnvalue false)
    (Variables|Default|SetMovementEnabled true)
    (Widget|SetRenderOpacity (Variables|Default|GetMousePromptWidget) 0.3)
    (Widget|SetRenderOpacity (Variables|Default|GetControlsDisplayWidget) 1.0)
    (else
      (Variables|/Script/Engine.PlayerController|SetbShowMouseCursor _returnvalue true)
      (Variables|Default|SetMovementEnabled false)
      (Widget|SetRenderOpacity (Variables|Default|GetMousePromptWidget) 1.0)
      (Widget|SetRenderOpacity (Variables|Default|GetControlsDisplayWidget) 0.0))))

(event Input|ActionEvents|InputActionSelect
  (params (Key :type Key%20Structure :default "None"))
  (:Pressed
    (bind _asplayer_controller (Utilities|Casting|CastToPlayerController (Pawn|GetController)))
    (if (.ReturnValue (Class|PlayerController|GetHitResultUnderCursorforObjects _asplayer_controller (Utilities|Array|MakeArray "ObjectTypeQuery2") true))
      (Utilities|Casting|CastToAtomComponent (.HitComponent (Collision|BreakHitResult (.HitResult (Class|PlayerController|GetHitResultUnderCursorforObjects _asplayer_controller (Utilities|Array|MakeArray "ObjectTypeQuery2") true)))))
      (Development|PrintString "Atom Clicked"))))

(event Input|ActionEvents|InputActionQuit
  (params (Key :type Key%20Structure :default "None"))
  (:Pressed
    (Game|QuitGame 0 "Quit" false)))

(event Input|AxisEvents|InputAxisForwardBackward
  (params (AxisValue :type Float%20%28single-precision%29))
  (if (Variables|Default|GetMovementEnabled)
    (Class|PawnMovementComponent|AddInputVector (Variables|Default|GetFloatingPawnMovement) (* (Math|Vector|GetForwardVector (Variables|Default|GetCamera)) AxisValue) false)))

(event Input|AxisEvents|InputAxisLookUp
  (params (AxisValue :type Float%20%28single-precision%29))
  (if (Variables|Default|GetMovementEnabled)
    (Pawn|Input|AddControllerPitchInput AxisValue)))

(event Input|AxisEvents|InputAxisTurn
  (params (AxisValue :type Float%20%28single-precision%29))
  (if (Variables|Default|GetMovementEnabled)
    (Pawn|Input|AddControllerYawInput AxisValue)))

(event Input|AxisEvents|InputAxisRightLeft
  (params (AxisValue :type Float%20%28single-precision%29))
  (if (Variables|Default|GetMovementEnabled)
    (Class|PawnMovementComponent|AddInputVector (Variables|Default|GetFloatingPawnMovement) (* (Math|Vector|GetRightVector (Variables|Default|GetCamera)) AxisValue) false)))

(fn ConstructionScript)